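; BP_BaseEnemy is a base enemy Blueprint driven by the Gameplay Ability System.
; On BeginPlay it applies the GE_InitPlayer effect to itself through its AbilitySystem, then prints a gameplay attribute value.
; Tick polls an attribute value every frame and destroys the actor when it equals exactly zero, rather than reacting to attribute-change events.
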(event `self.ReceiveBeginPlay`
  (`AbilitySystemComponent.BP_ApplyGameplayEffectToSelf` :`self` (`self.AbilitySystem`) :`GameplayEffectClass` "/Game/Babylon/Blueprints/Effects/GE_InitPlayer.GE_InitPlayer_C")
  (`KismetSystemLibrary.PrintText` (`KismetTextLibrary.Conv_DoubleToText` (`.ReturnValue` (`AbilitySystemComponent.GetGameplayAttributeValue` (`self.AbilitySystem`) (struct :`AttributeName` "HP" :`Attribute` "/Script/Babylon.BabylonAttributeSet:HP" :`AttributeOwner` "/Script/CoreUObject.Class'/Script/Babylon.BabylonAttributeSet'"))) "HalfToEven")))

(event `self.ReceiveTick`
  (params (DeltaSeconds :type "Float (single-precision)"))
  (if (== (`.ReturnValue` (`AbilitySystemComponent.GetGameplayAttributeValue` (`self.AbilitySystem`) (struct :`AttributeName` "HP" :`Attribute` "/Script/Babylon.BabylonAttributeSet:HP" :`AttributeOwner` "/Script/CoreUObject.Class'/Script/Babylon.BabylonAttributeSet'"))) 0.0)
    (`self.K2_DestroyActor`)))

(fn `UserConstructionScript`)