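; GA_Attack is a Gameplay Ability that performs a single-target melee attack in front of the avatar.
; On activation it commits, then sphere-traces a short distance forward for the first pawn hit.
; DamageFunction combines attacker strength attributes with target defense and block into a negative magnitude, applied through GE_Damage via SetByCaller.
; Debug prints and trace drawing remain, and the ability only ends when a valid target is hit.
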(event `self.K2_ActivateAbility`
  (bind _returnvalue (`AbilitySystemBlueprintLibrary.GetAbilitySystemComponent` (`self.Player`)))
  (bind _returnvalue_2 (`AbilitySystemBlueprintLibrary.GetAbilitySystemComponent` (`self.Target`)))
  (bind _output_get (set `self.Player` (`self.GetAvatarActorFromActorInfo`)))
  (`self.K2_CommitAbility`)
  (if true
    (`KismetSystemLibrary.PrintString` "ATTACK")
    (bind _returnvalue_3 (`Actor.K2_GetActorLocation` _output_get))
    (bind _outhit (`KismetSystemLibrary.SphereTraceSingleForObjects` _returnvalue_3 (+ _returnvalue_3 (* (`Actor.GetActorForwardVector` _output_get) 100.0)) 50.0 (`|MakeArray` "ObjectTypeQuery3" :!type "EObjectTypeQuery Enum") false (`|MakeArray` _output_get) "ForDuration" :!pinned true)) ; TODO: Make it possible to hit multiple enemies at once
    (bind (_bblockinghit _binitialoverlap _time _distance _location _impactpoint _normal _impactnormal _physmat _hitactor) (`GameplayStatics.BreakHitResult` _outhit))
    (bind _output_get_2 (set `self.Target` _hitactor))
    (if (`KismetSystemLibrary.IsValid` _output_get_2)
      (bind _damage (`self.DamageFunction` (`.ReturnValue` (`AbilitySystemComponent.GetGameplayAttributeValue` _returnvalue (struct :`AttributeName` "WStr" :`Attribute` "/Script/Babylon.BabylonAttributeSet:WStr" :`AttributeOwner` "/Script/CoreUObject.Class'/Script/Babylon.BabylonAttributeSet'"))) (`.ReturnValue` (`AbilitySystemComponent.GetGameplayAttributeValue` _returnvalue (struct :`AttributeName` "AStr" :`Attribute` "/Script/Babylon.BabylonAttributeSet:AStr" :`AttributeOwner` "/Script/CoreUObject.Class'/Script/Babylon.BabylonAttributeSet'"))) (`.ReturnValue` (`AbilitySystemComponent.GetGameplayAttributeValue` _returnvalue_2 (struct :`AttributeName` "Def" :`Attribute` "/Script/Babylon.BabylonAttributeSet:Def" :`AttributeOwner` "/Script/CoreUObject.Class'/Script/Babylon.BabylonAttributeSet'"))) (`.ReturnValue` (`AbilitySystemComponent.GetGameplayAttributeValue` _returnvalue_2 (struct :`AttributeName` "Block" :`Attribute` "/Script/Babylon.BabylonAttributeSet:Block" :`AttributeOwner` "/Script/CoreUObject.Class'/Script/Babylon.BabylonAttributeSet'")))))
      (bind _returnvalue_4 (`AbilitySystemBlueprintLibrary.AssignTagSetByCallerMagnitude` (`self.MakeOutgoingGameplayEffectSpec` "/Game/Babylon/Blueprints/Effects/GE_Damage.GE_Damage_C") (struct :`TagName` "Damage") _damage))
      (`self.K2_ApplyGameplayEffectSpecToTarget` _returnvalue_4 (`AbilitySystemBlueprintLibrary.AbilityTargetDataFromActor` _hitactor))
      (`KismetSystemLibrary.PrintString` (`KismetStringLibrary.Conv_DoubleToString` (`.ReturnValue` (`AbilitySystemComponent.GetGameplayAttributeValue` (`AbilitySystemBlueprintLibrary.GetAbilitySystemComponent` (`self.Target`)) (struct :`AttributeName` "HP" :`Attribute` "/Script/Babylon.BabylonAttributeSet:HP" :`AttributeOwner` "/Script/CoreUObject.Class'/Script/Babylon.BabylonAttributeSet'")))))
      (`self.K2_EndAbility`))
    (else
      (`self.K2_CancelAbility`))))

(fn `DamageFunction`
  (params (WeaponStr :type "Float (double-precision)") (AttackStr :type "Float (double-precision)") (TargetDef :type "Float (double-precision)") (TargetBlock :type "Float (double-precision)"))
  (returns (Damage :type "Float (double-precision)"))
  (return (* (- (* (* WeaponStr AttackStr) (- 1.0 TargetDef)) TargetBlock) -1.0)))